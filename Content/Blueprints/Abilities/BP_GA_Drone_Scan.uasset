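; Gameplay ability for a drone scan that shows a scan wave effect at the avatar's location.
; On activation it spawns the NS_ScanWave Niagara system and passes its color, radius and speed variables into the system's User parameters.
; The graph holds only the visual, with no detection logic or End Ability call, and the node feeding highlight duration to the effect is disconnected.
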(event `self.K2_ActivateAbility`
  (bind _returnvalue (`NiagaraFunctionLibrary.SpawnSystemAtLocation` "/Game/Art/NS_ScanWave.NS_ScanWave" (`Actor.K2_GetActorLocation` (`self.GetAvatarActorFromActorInfo`))))
  (set `self.NS` _returnvalue)
  (`NiagaraComponent.SetVariableLinearColor` (`self.NS`) "User.ScanColor" (`self.ScanColor`))
  (`NiagaraComponent.SetVariableFloat` (`self.NS`) "User.ScanRadius" (`self.ScanRadius`))
  (`NiagaraComponent.SetVariableFloat` (`self.NS`) "User.ScanSpeed" (`self.ScanSpeed`)))