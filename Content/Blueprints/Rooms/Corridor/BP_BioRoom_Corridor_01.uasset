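; Corridor room Blueprint that opens or seals each of its four sides according to a door configuration.
; ApplyDoorConfig passes the North, East, South and West flags to SetVisibilityAndCollision with that side's wall and door frame meshes.
; The helper shows and enables collision on the door frame for an open side, or on the wall for a closed one, disabling the other.
; Older wall-only branches remain in the event graph, unconnected.
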(event `self.ApplyDoorConfig`
  (params (Doors :type "SignalRoomDoors Structure (by ref)"))
  (`|ExecutionSequence`
    (:`then_0`
      (`self.SetVisibilityAndCollision` (`self.SM_Wall_North`) (`self.SM_DoorFrame_North`) Doors_bNorth))
    (:`then_1`
      (`self.SetVisibilityAndCollision` (`self.SM_Wall_East`) (`self.SM_DoorFrame_East`) Doors_bEast))
    (:`then_2`
      (`self.SetVisibilityAndCollision` (`self.SM_Wall_South`) (`self.SM_DoorFrame_South`) Doors_bSouth))
    (:`then_3`
      (`self.SetVisibilityAndCollision` (`self.SM_Wall_West`) (`self.SM_DoorFrame_West`) Doors_bWest))))

(fn `UserConstructionScript`)