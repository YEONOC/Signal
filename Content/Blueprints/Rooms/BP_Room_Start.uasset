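; BP_Room_Start is a room Blueprint, apparently the start room, that opens or closes its four sides from a door configuration.
; Its construction script calls MergeWall per side to clear that wall's HISM and add instances from tagged static mesh transforms.
; MergeWall returns inside its loop, so only the first tagged mesh is added.
; ApplyDoorConfig hides a side's entire HISM where a door is set, otherwise shows it.
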(event `self.ApplyDoorConfig`
  (params (Doors :type "SignalRoomDoors Structure (by ref)"))
  (`|ExecutionSequence`
    (:`then_0`
      (if Doors_bNorth
        (`SceneComponent.SetVisibility` (`self.Wall_North_HISM`) false false)
        (else
          (`SceneComponent.SetVisibility` (`self.Wall_North_HISM`) true true))))
    (:`then_1`
      (if Doors_bEast
        (`SceneComponent.SetVisibility` (`self.Wall_East_HISM`) false false)
        (else
          (`SceneComponent.SetVisibility` (`self.Wall_East_HISM`) true true))))
    (:`then_2`
      (if Doors_bSouth
        (`SceneComponent.SetVisibility` (`self.Wall_South_HISM`) false false)
        (else
          (`SceneComponent.SetVisibility` (`self.Wall_South_HISM`) true true))))
    (:`then_3`
      (if Doors_bWest
        (`SceneComponent.SetVisibility` (`self.Wall_West_HISM`) false false)
        (else
          (`SceneComponent.SetVisibility` (`self.Wall_West_HISM`) true true))))))

(fn `UserConstructionScript`
  (`|ExecutionSequence`
    (:`then_0`
      (`self.MergeWall` (`self.Wall_East_HISM`) "Wall_East"
        (:`Return`
          (`self.MergeWall` (`self.Wall_West_HISM`) "Wall_West"
            (:`Return`
              (`self.MergeWall` (`self.Wall_North_HISM`) "Wall_North"
                (:`Return`
                  (`self.MergeWall` (`self.Wall_South_HISM`) "Wall_South"))))))))))